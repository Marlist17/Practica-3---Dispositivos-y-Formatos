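; BP_Diana is a dartboard that scores thrown darts and shows the running total.
; When its cylinder mesh is hit by a BP_Dardos, it calls a keep-world attach with the dart's root as parent and stops the dart's physics simulation.
; Overlap checks on the Centro and ZonaMedia zones pick the points, with a lower score for other hits, and update the TextRender.
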(event `self.SM_DartboardDarts_Cylinder.OnComponentHit`
  (params (HitComponent :type "PrimitiveComponent Object Reference") (OtherActor :type "Actor Object Reference") (OtherComp :type "PrimitiveComponent Object Reference") (NormalImpulse :type "Vector Structure") (Hit :type "HitResult Structure (by ref)"))
  (bind _asbp_dardos (cast `/Game/mesh/dardos/BP_Dardos` OtherActor))
  (set `self.BP Dardos` _asbp_dardos)
  (`self.K2_AttachToComponent` self (`Actor.RootComponent` (`self.BP Dardos`)) "None" "KeepWorld" "KeepWorld" "KeepWorld" true)
  (`PrimitiveComponent.SetSimulatePhysics` (`/Game/mesh/dardos/BP_Dardos.SM_DartboardDarts_Cylinder_001` (`self.BP Dardos`)) false)
  (if (`PrimitiveComponent.IsOverlappingActor` (`self.Centro`) (`self.BP Dardos`))
    (bind _output_get (set `self.Puntos` (+ (`self.Puntos`) 100)))
    (`TextRenderComponent.K2_SetText` (`self.TextRender`) (`KismetTextLibrary.Conv_IntToText` _output_get))
    (elif (`PrimitiveComponent.IsOverlappingActor` (`self.Zona media`) (`self.BP Dardos`))
      (bind _output_get_2 (set `self.Puntos` (+ (`self.Puntos`) 50)))
      (`TextRenderComponent.K2_SetText` (`self.TextRender`) (`KismetTextLibrary.Conv_IntToText` _output_get_2))
      (else
        (bind _output_get_3 (set `self.Puntos` (+ (`self.Puntos`) 30)))
        (`TextRenderComponent.K2_SetText` (`self.TextRender`) (`KismetTextLibrary.Conv_IntToText` _output_get_3))))))

(fn `UserConstructionScript`)